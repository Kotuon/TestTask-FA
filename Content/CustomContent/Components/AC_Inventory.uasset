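; Actor component that gives BP_FirstPersonCharacter a size-limited item inventory and caches the character's HUD reference on BeginPlay.
; AddToInventory appends an item while a slot is free, returning false when full.
; On success it re-fetches W_Hud from the owner's HUD widget to show the item's image at the new index.
; The picked-up actor is teleported far out of the playable space rather than destroyed, keeping stored references valid.
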(event `self.ReceiveBeginPlay`
  (bind _asbp_first_person_character (cast `/Game/FirstPerson/Blueprints/BP_FirstPersonCharacter` (`self.GetOwner`)))
  (set `self.hudRef` (`/Game/FirstPerson/Blueprints/BP_FirstPersonCharacter.hudRef` _asbp_first_person_character)))

(fn `AddToInventory`
  (params (newItem :type "/Game/CustomContent/Interactable/BP_Item Object Reference"))
  (returns (`success?` :type Boolean))
  (locals (l_newItem :type "/Game/CustomContent/Interactable/BP_Item Object Reference"))
  (bind _itemlist (`self.itemList`))
  (set `local.l_newItem` newItem)
  (if (<= (`KismetArrayLibrary.Array_Length` _itemlist) (- (`self.inventorySize`) 1))
    (`KismetArrayLibrary.Array_Add` _itemlist (`local.l_newItem`))
    (bind _asbp_first_person_character (cast `/Game/FirstPerson/Blueprints/BP_FirstPersonCharacter` (`self.GetOwner`)))
    (bind _asw_hud (cast `/Game/CustomContent/UI/W_Hud` (`WidgetComponent.GetWidget` (`/Game/FirstPerson/Blueprints/BP_FirstPersonCharacter.HUD` _asbp_first_person_character))))
    (`/Game/CustomContent/UI/W_Hud.UpdateImage` _asw_hud (`/Game/CustomContent/Interactable/BP_Item.inventoryImage` (`local.l_newItem`)) (- (`KismetArrayLibrary.Array_Length` (`self.itemList`)) 1))
    (`Actor.K2_SetActorLocation` (`local.l_newItem`) (-10000.0 -10000.0 -10000.0) false true)
    (return true)
    (else
      (return false))))