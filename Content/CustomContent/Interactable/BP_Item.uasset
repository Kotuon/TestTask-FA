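; BP_Item is an interactable item that the player can add to their inventory.
; Interact passes the actor itself to the player's ACInventory component.
; If the add fails, it shows an inventory-full message on the widget and starts a timer to call ResetText.
; ResetText restores the interact prompt if the player is still in radius and able to interact, otherwise it clears the text.
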(fn `Interact`
  (bind _success_ (`/Game/CustomContent/Components/AC_Inventory.AddToInventory` (`/Game/FirstPerson/Blueprints/BP_FirstPersonCharacter.AC_Inventory` (`self.playerRef`)) self))
  (if (not _success_)
    (`self.UpdateWidget` "Inventory full!")
    (`KismetSystemLibrary.K2_SetTimer` null "ResetText" 2.0)))

(fn `ResetText`
  (if (and (`self.playerCanInteract`) (`self.playerInRadius`))
    (`self.UpdateWidget` (`self.interactMessage`))
    (else
      (`self.UpdateWidget` ""))))

(fn `UserConstructionScript`
  (`parent.UserConstructionScript`))