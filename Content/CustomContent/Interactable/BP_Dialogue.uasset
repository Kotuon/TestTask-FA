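; BP_Dialogue is an interactable that shows typewriter-style dialogue in a W_Dialogue widget created on BeginPlay.
; Interact opens the box, switches the first-person character to menu input and shows the cursor.
; Tick reveals each sentence character by character, using a short Delay as a throttle.
; SkipText completes or advances sentences, then ExitText restores game input; TextOver stays set, so the dialogue plays only once.
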(event `self.ReceiveBeginPlay`
  (`parent.ReceiveBeginPlay`)
  (bind _returnvalue (`|CreateWidget` "/Game/CustomContent/UI/W_Dialogue.W_Dialogue_C"))
  (bind _output_get (set `self.dialogueRef` _returnvalue))
  (set `/Game/CustomContent/UI/W_Dialogue.actorRef` self _output_get)
  (`UserWidget.AddToViewport` _output_get 0))

(event `self.ReceiveTick`
  (params (DeltaSeconds :type "Float (single-precision)"))
  (bind _output (`|GetArrayItem` (`self.dialogueText`) (`self.sentenceIndex`)))
  (bind _skiptext (`/Game/CustomContent/UI/W_Dialogue.SkipText` (`self.dialogueRef`)))
  (`parent.ReceiveTick` DeltaSeconds)
  (if (and (`self.talking?`) (`self.nextText?`))
    (set `self.currStringLength` (`KismetStringLibrary.Len` _output))
    (`TextBlock.SetText` (`/Game/CustomContent/UI/W_Dialogue.DialogueText` (`self.dialogueRef`)) (`KismetTextLibrary.Conv_StringToText` (`KismetStringLibrary.GetSubstring` _output 0 (`self.currStringIndex`))))
    (`KismetSystemLibrary.Delay` 0.025)
    (if (>= (`self.currStringIndex`) (`self.currStringLength`))
      (set `self.nextText?` false)
      (if (< (+ (`self.sentenceIndex`) 1) (`KismetArrayLibrary.Array_Length` (`self.dialogueText`)))
        (`TextBlock.SetText` _skiptext "Next")
        (else
          (`TextBlock.SetText` _skiptext "Close")
          (set `self.textOver?` true)))
      (else
        (`/Engine/EditorBlueprintResources/StandardMacros.IncrementInt` (`self.currStringIndex`))))))

(fn `ExitText`
  (bind _returnvalue (`GameplayStatics.GetPlayerController` 0))
  (`Widget.SetVisibility` (`/Game/CustomContent/UI/W_Dialogue.DialogueBoxCanvas` (`self.dialogueRef`)) "Hidden")
  (`Widget.SetVisibility` (`/Game/CustomContent/UI/W_InteractMessage.MyMessage` (`self.interactMessageRef`)) "Hidden")
  (set `self.talking?` false)
  (bind _asbp_first_person_character (cast `/Game/FirstPerson/Blueprints/BP_FirstPersonCharacter` (`GameplayStatics.GetPlayerCharacter` 0)))
  (`TestTaskFACharacter.SetInputStatus` _asbp_first_person_character "IS_Game")
  (`WidgetBlueprintLibrary.SetInputMode_GameOnly` _returnvalue)
  (set `PlayerController.bShowMouseCursor` false _returnvalue))

(fn `Interact`
  (bind _returnvalue (`GameplayStatics.GetPlayerController` 0))
  (`parent.Interact`)
  (if (and (not (`self.talking?`)) (not (`self.textOver?`)))
    (`Widget.SetVisibility` (`/Game/CustomContent/UI/W_Dialogue.DialogueBoxCanvas` (`self.dialogueRef`)) "Visible")
    (`Widget.SetVisibility` (`/Game/CustomContent/UI/W_InteractMessage.MyMessage` (`self.interactMessageRef`)) "Hidden")
    (set `self.talking?` true)
    (bind _asbp_first_person_character (cast `/Game/FirstPerson/Blueprints/BP_FirstPersonCharacter` (`GameplayStatics.GetPlayerCharacter` 0)))
    (`TestTaskFACharacter.SetInputStatus` _asbp_first_person_character "IS_Menu")
    (set `self.nextText?` true)
    (`WidgetBlueprintLibrary.SetInputMode_GameAndUIEx` _returnvalue (`self.dialogueRef`) "DoNotLock" false)
    (set `PlayerController.bShowMouseCursor` true _returnvalue)
    (set `self.textOver?` false)
    (else
      (`self.SkipText`))))

(fn `SkipText`
  (if (`self.textOver?`)
    (`self.ExitText`)
    (elif (< (`self.currStringIndex`) (`self.currStringLength`))
      (set `self.currStringIndex` (`self.currStringLength`))
      (elif (not (`self.nextText?`))
        (set `self.nextText?` true)
        (set `self.currStringIndex` 1)
        (bind _result (`/Engine/EditorBlueprintResources/StandardMacros.IncrementInt` (`self.sentenceIndex`))
          (:`  `
            (if (>= _result (`KismetArrayLibrary.Array_Length` (`self.dialogueText`)))
              (set `self.talking?` false)
              (set `self.textOver?` true)
              (`TextBlock.SetText` (`/Game/CustomContent/UI/W_Dialogue.SkipText` (`self.dialogueRef`)) "Close"))))))))

(fn `UserConstructionScript`
  (`parent.UserConstructionScript`))