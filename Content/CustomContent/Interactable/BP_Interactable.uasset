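; BP_Interactable is an interactable actor that shows a prompt when a nearby player looks toward it.
; InRange and OutRange set player proximity; the Sphere overlap events are empty.
; While in range, Tick compares the dot product of camera forward and player-to-actor direction to a threshold.
; The result sets PlayerCanInteract and shows or clears the widget message; Interact is an empty stub.
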(event `self.ReceiveBeginPlay`
  (bind _asw_interact_message (cast `/Game/CustomContent/UI/W_InteractMessage` (`WidgetComponent.GetWidget` (`self.W_InteractMessage`))))
  (set `self.interactMessageRef` _asw_interact_message))

(event `self.ReceiveTick`
  (params (DeltaSeconds :type "Float (single-precision)"))
  (if (`self.playerInRadius`)
    (bind _returnvalue (`self.GetPlayerLookAngle`))
    (if (>= _returnvalue 0.8)
      (set `self.playerCanInteract` true)
      (`self.UpdateWidget` (`self.interactMessage`))
      (else
        (set `self.playerCanInteract` false)
        (`self.UpdateWidget` "")))))

(event `self.Sphere.OnComponentBeginOverlap`
  (params (OverlappedComponent :type "PrimitiveComponent Object Reference") (OtherActor :type "Actor Object Reference") (OtherComp :type "PrimitiveComponent Object Reference") (OtherBodyIndex :type Integer) (bFromSweep :type Boolean) (SweepResult :type "HitResult Structure (by ref)")))

(event `self.Sphere.OnComponentEndOverlap`
  (params (OverlappedComponent :type "PrimitiveComponent Object Reference") (OtherActor :type "Actor Object Reference") (OtherComp :type "PrimitiveComponent Object Reference") (OtherBodyIndex :type Integer)))

(fn `GetPlayerLookAngle`
  (returns (ReturnValue :type "Float (double-precision)"))
  (return (`KismetMathLibrary.Dot_VectorVector` (`SceneComponent.GetForwardVector` (`TestTaskFACharacter.FirstPersonCameraComponent` (`self.playerRef`))) (`KismetMathLibrary.Normal` (- (`self.K2_GetActorLocation`) (`self.K2_GetActorLocation` (`self.playerRef`)))))))

(fn `InRange`
  (params (player :type "/Game/FirstPerson/Blueprints/BP_FirstPersonCharacter Object Reference"))
  (set `self.playerRef` player)
  (set `self.playerInRadius` true))

(fn `Interact`)

(fn `OutRange`
  (set `self.playerInRadius` false)
  (set `self.playerCanInteract` false)
  (`self.UpdateWidget` ""))

(fn `UpdateWidget`
  (params (message :type Text))
  (bind _asw_interact_message (cast `/Game/CustomContent/UI/W_InteractMessage` (`WidgetComponent.GetUserWidgetObject` (`self.W_InteractMessage`))))
  (set `TextBlock.Text` message (`/Game/CustomContent/UI/W_InteractMessage.MyMessage` _asw_interact_message)))

(fn `UserConstructionScript`)